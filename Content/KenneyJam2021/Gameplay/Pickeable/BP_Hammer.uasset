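; Hammer pickup for the KenneyJam2021 game that the player collects into their inventory by interacting with it.
; Interact calls the parent implementation, then passes ItemName to AddItemToInventory on PC_KenneyJam2021, obtained from player controller 0.
; The actor destroys itself only when that call succeeds, so a failed add leaves the hammer in the world.
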(event EventBeginPlay
  (|CallParentFunction) ; This node is disabled and will not be called.\nDrag off pins to build functionality.
)

(event Collision|EventActorBeginOverlap
  (params (OtherActor :type Actor%20Object%20Reference))
  (|CallParentFunction OtherActor) ; This node is disabled and will not be called.\nDrag off pins to build functionality.
)

(event EventTick
  (params (DeltaSeconds :type Float%20%28single-precision%29)))

(event EventInteract
  (|CallParentFunction)
  (bind _aspc_kenney_jam_2021 (Utilities|Casting|CastToPC_KenneyJam2021 (Game|GetPlayerController 0)))
  (bind _successful (Default|AddItemtoInventory _aspc_kenney_jam_2021 (Variables|Default|GetItemName)))
  (if _successful
    (Actor|DestroyActor)))

(fn ConstructionScript
  (|CallParentFunction))