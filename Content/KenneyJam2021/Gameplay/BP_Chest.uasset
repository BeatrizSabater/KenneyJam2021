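; BP_Chest is an interactable chest that asks the player controller, PC_KenneyJam2021, to open it.
; Its Box overlap events register and unregister the chest with the overlapping actor's AC_Interact component.
; The Interact event prints a debug string and calls OpenChest on the controller.
; Every tick, its TextRender turns to face the isometric camera pawn's location.
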(event OnComponentBeginOverlap(Box)
  (params (OverlappedComponent :type Primitive%20Component%20Object%20Reference) (OtherActor :type Actor%20Object%20Reference) (OtherComp :type Primitive%20Component%20Object%20Reference) (OtherBodyIndex :type Integer) (bFromSweep :type Boolean) (SweepResult :type Hit%20Result%20Structure%20%28by%20ref%29))
  (Default|OverlapInteractuableObject (Actor|GetComponentbyClass OtherActor "/Game/KenneyJam2021/Core/AC_Interact.AC_Interact_C") self))

(event OnComponentEndOverlap(Box)
  (params (OverlappedComponent :type Primitive%20Component%20Object%20Reference) (OtherActor :type Actor%20Object%20Reference) (OtherComp :type Primitive%20Component%20Object%20Reference) (OtherBodyIndex :type Integer))
  (Default|EndOverlapInteractuableObject (Actor|GetComponentbyClass OtherActor "/Game/KenneyJam2021/Core/AC_Interact.AC_Interact_C") self))

(event EventBeginPlay)

(event Collision|EventActorBeginOverlap
  (params (OtherActor :type Actor%20Object%20Reference)))

(event EventInteract
  (Development|PrintString "Interacting with chest.")
  (bind _aspc_kenney_jam_2021 (Utilities|Casting|CastToPC_KenneyJam2021 (Game|GetPlayerController 0)))
  (Default|OpenChest _aspc_kenney_jam_2021))

(event EventTick
  (params (DeltaSeconds :type Float%20%28single-precision%29))
  (Transformation|SetWorldRotation (Variables|Default|GetTextRender) (Math|Rotator|FindLookatRotation (Transformation|GetWorldLocation (Variables|Default|GetTextRender)) (Transformation|GetActorLocation (.AsBP%20Isometric%20Camera%20Pawn (Utilities|Casting|CastToBP_IsometricCameraPawn (Game|Player|GetPlayerPawn 0))))) false false))

(fn ConstructionScript)