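; Chalice pickup event that gives the player a "Chalice" inventory item in exchange for a needed object.
; Destroys itself on BeginPlay when the game instance's RespawnChalice flag is off.
; Overlapping its box as the Yennek character opens a hint dialog that something is missing.
; DoThings consumes the needed object, adds the Chalice, unhides the first referenced actor, and clears the respawn flag if the add succeeds.
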(event OnComponentBeginOverlap(Box)
  (params (OverlappedComponent :type Primitive%20Component%20Object%20Reference) (OtherActor :type Actor%20Object%20Reference) (OtherComp :type Primitive%20Component%20Object%20Reference) (OtherBodyIndex :type Integer) (bFromSweep :type Boolean) (SweepResult :type Hit%20Result%20Structure%20%28by%20ref%29))
  (Utilities|Casting|CastToBP_YennekCharacter OtherActor)
  (CallFunction|OpenDialogText "Hm... Feels like it is missing something."))

(event EventBeginPlay
  (|CallParentFunction)
  (if (not (Variables|/Game/KenneyJam2021/Core/Framework/GI_KenneyJam2021.GI_KenneyJam2021_C|GetbRespawnChalice (.AsGI%20Kenney%20Jam%202021 (Utilities|Casting|CastToGI_KenneyJam2021 (Game|GetGameInstance)))))
    (Actor|DestroyActor)))

(event Collision|EventActorBeginOverlap
  (params (OtherActor :type Actor%20Object%20Reference))
  (|CallParentFunction OtherActor))

(event EventTick
  (params (DeltaSeconds :type Float%20%28single-precision%29))
  (|CallParentFunction DeltaSeconds) ; This node is disabled and will not be called.\nDrag off pins to build functionality.
)

(event EventDoThings
  (CallFunction|RemoveItemfromInventory (Variables|Default|GetNeededObject))
  (bind _aspc_kenney_jam_2021 (Utilities|Casting|CastToPC_KenneyJam2021 (Game|GetPlayerController 0)))
  (bind _successful (Default|AddItemtoInventory _aspc_kenney_jam_2021 "Chalice"))
  (Rendering|SetActorHiddenInGame (Utilities|Array|Get(acopy) (Variables|Default|GetReferencedActors)) false)
  (if _successful
    (Variables|/Game/KenneyJam2021/Core/Framework/GI_KenneyJam2021.GI_KenneyJam2021_C|SetbRespawnChalice (.AsGI%20Kenney%20Jam%202021 (Utilities|Casting|CastToGI_KenneyJam2021 (Game|GetGameInstance))) false)))

(fn ConstructionScript
  (|CallParentFunction))