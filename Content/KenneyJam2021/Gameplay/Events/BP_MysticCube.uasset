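; Mystic cube actor for the Kenney Jam 2021 game, with visibility tied to the chalice respawn state.
; On BeginPlay it reads RespawnChalice from GI_KenneyJam2021 and sets itself visible in game when that flag is false.
; An unconnected branch holds a similar check against the current level's RespawnItems flag, found by level name, and never runs.
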(event EventBeginPlay
  (if (not (Variables|/Game/KenneyJam2021/Core/Framework/GI_KenneyJam2021.GI_KenneyJam2021_C|GetbRespawnChalice (.AsGI%20Kenney%20Jam%202021 (Utilities|Casting|CastToGI_KenneyJam2021 (Game|GetGameInstance)))))
    (Rendering|SetActorHiddenInGame false)))

(event Collision|EventActorBeginOverlap
  (params (OtherActor :type Actor%20Object%20Reference)))

(event EventTick
  (params (DeltaSeconds :type Float%20%28single-precision%29)))

(fn ConstructionScript)