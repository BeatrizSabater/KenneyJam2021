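; BP_JustText is a trigger actor that shows a one-time dialogue text when the player character walks into its box.
; On BeginPlay it destroys itself if the game instance's respawn flag matching its MyName item (Axe, Hammer, Mystic Cube, Wheat or Windmill) is false.
; On overlap it opens the dialogue only if the current level's entry has RespawnItems set and the text has not been shown yet.
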(event OnComponentBeginOverlap(Box)
  (params (OverlappedComponent :type Primitive%20Component%20Object%20Reference) (OtherActor :type Actor%20Object%20Reference) (OtherComp :type Primitive%20Component%20Object%20Reference) (OtherBodyIndex :type Integer) (bFromSweep :type Boolean) (SweepResult :type Hit%20Result%20Structure%20%28by%20ref%29))
  (Utilities|Casting|CastToBP_YennekCharacter OtherActor)
  (bind _returnvalue (Game|GetCurrentLevelName true))
  (bind _smap (CallFunction|FindLevelbyName (CallFunction|GetLevels) _returnvalue))
  (if (and (.RespawnItems (Utilities|Struct|BreakSMap _smap)) (not (Variables|Default|GetbHasBeenShown)))
    (CallFunction|OpenDialogText (Variables|Default|GetDialogueText))
    (Variables|Default|SetbHasBeenShown true)))

(event EventBeginPlay
  (bind _returnvalue (Game|GetGameInstance))
  (bind _asgi_kenney_jam_2021 (Utilities|Casting|CastToGI_KenneyJam2021 _returnvalue))
  (switch name (Variables|Default|GetMyName)
    (:Axe
      (if (not (Variables|/Game/KenneyJam2021/Core/Framework/GI_KenneyJam2021.GI_KenneyJam2021_C|GetbRespawnAxe _asgi_kenney_jam_2021))
        (Actor|DestroyActor :!label _label)))
    (:Hammer
      (if (not (Variables|/Game/KenneyJam2021/Core/Framework/GI_KenneyJam2021.GI_KenneyJam2021_C|GetbRespawnHammer _asgi_kenney_jam_2021))
        (goto _label)))
    (:MysticCube
      (if (not (Variables|/Game/KenneyJam2021/Core/Framework/GI_KenneyJam2021.GI_KenneyJam2021_C|GetbRespawnMysticBlock _asgi_kenney_jam_2021))
        (goto _label)))
    (:Wheat
      (if (not (Variables|/Game/KenneyJam2021/Core/Framework/GI_KenneyJam2021.GI_KenneyJam2021_C|GetbRespawnWheat _asgi_kenney_jam_2021))
        (goto _label)))
    (:Windmill
      (if (not (Variables|/Game/KenneyJam2021/Core/Framework/GI_KenneyJam2021.GI_KenneyJam2021_C|GetbRespawnWindmill _asgi_kenney_jam_2021))
        (goto _label)))))

(fn ConstructionScript)