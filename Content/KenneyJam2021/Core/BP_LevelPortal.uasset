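; BP_LevelPortal is a level transition portal that loads the neighbouring map when an actor overlaps it.
; On BeginPlay it asks GI_KenneyJam2021 for the next map, using the current level name and the portal's Orientation.
; On overlap it opens that map by name after a short delay with a debug print, or only prints a warning if the map is "Void".
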(event EventBeginPlay
  (bind _asgi_kenney_jam_2021 (Utilities|Casting|CastToGI_KenneyJam2021 (Game|GetGameInstance)))
  (bind _returnvalue (Game|GetCurrentLevelName true))
  (bind _nextmap (Default|GetBridgeNextMap _asgi_kenney_jam_2021 _returnvalue (Variables|Default|GetOrientation)))
  (Variables|Default|SetNextMap _nextmap))

(event Collision|EventActorBeginOverlap
  (params (OtherActor :type Actor%20Object%20Reference))
  (bind _nextmap (Variables|Default|GetNextMap))
  (if (Utilities|Enum|NotEqual(Enum) (Variables|Default|GetNextMap) "Void")
    (Development|PrintString (Utilities|String|Append "Opening level to: " _nextmap))
    (Utilities|FlowControl|Delay 2.0)
    (Game|OpenLevel(byName) (Utilities|String|StringToName _nextmap))
    (else
      (Development|PrintString "VOID VOID VOID VOID"))))

(fn ConstructionScript)