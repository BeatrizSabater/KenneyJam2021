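; BP_PickableObject is an interactable world actor, named as a pickup, for a Kenney Jam 2021 game.
; On overlap begin and end, it registers or unregisters itself with the other actor's AC_Interact component, if present.
; Its Interact event only prints the object's name, as do the overlap handlers for debugging, so no pickup logic is implemented here.
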(event EventBeginPlay)

(event Collision|EventActorBeginOverlap
  (params (OtherActor :type Actor%20Object%20Reference))
  (bind _returnvalue (Actor|GetComponentbyClass OtherActor "/Game/KenneyJam2021/Core/AC_Interact.AC_Interact_C"))
  (Utilities|IsValid _returnvalue
    (:Is%20Valid
      (Default|OverlapInteractuableObject _returnvalue self)
      (Development|PrintString (Utilities|String|Append "Begin overlap: " (Utilities|GetDisplayName self))))))

(event Collision|EventActorEndOverlap
  (params (OtherActor :type Actor%20Object%20Reference))
  (bind _returnvalue (Actor|GetComponentbyClass OtherActor "/Game/KenneyJam2021/Core/AC_Interact.AC_Interact_C"))
  (Utilities|IsValid _returnvalue
    (:Is%20Valid
      (Default|EndOverlapInteractuableObject _returnvalue self)
      (Development|PrintString (Utilities|String|Append "End overlap: " (Utilities|GetDisplayName self))))))

(event EventInteract
  (Development|PrintString (Utilities|String|Append "Interacting with: " (Utilities|GetDisplayName self))))

(fn ConstructionScript)