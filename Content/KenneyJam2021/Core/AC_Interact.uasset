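; AC_Interact is an interaction component that tracks the object currently available to interact with and triggers it.
; Overlap events store that object and bind to its OnDestroyed delegate, while end-overlap clears the reference only if it matches the stored one.
; Interact sends InteractMessage to the stored object, leaving the response to that object.
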(event Custom|OverlapInteractuableObject
  (params (CurrentInteractuableObject :type Actor%20Object%20Reference))
  (Variables|Default|SetCurrentInteractuableObject CurrentInteractuableObject)
  (Game|BindEventtoOnDestroyed CurrentInteractuableObject (EventDispatchers|CreateEvent :!event Custom|EndOverlapInteractuableObject)))

(event Custom|EndOverlapInteractuableObject
  (params (CurrentInteractuableObject :type Actor%20Object%20Reference))
  (if (== CurrentInteractuableObject (Variables|Default|GetCurrentInteractuableObject))
    (Variables|Default|SetCurrentInteractuableObject 0)))

(event Custom|Interact
  (Class|BPIInteractuable|Interact(Message) (Variables|Default|GetCurrentInteractuableObject)))

(event EventBeginPlay)

(event EventTick
  (params (DeltaSeconds :type Float%20%28single-precision%29)))