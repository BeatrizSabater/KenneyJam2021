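; Player controller for the main menu that starts the game by loading the Basecamp level.
; On BeginPlay it hides the cursor, shows the W_MainMenu widget and sets game-only input.
; A Gate holds back the Interact press until the menu's animation-finished event opens it, after which pressing Interact loads the level.
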(event Custom|OpenGate
  (Utilities|FlowControl|Gate true) ; enters at Open
)

(event EventBeginPlay
  (Variables|Default|SetbShowMouseCursor false)
  (bind _returnvalue (UserInterface|CreateWidget "/Game/KenneyJam2021/UI/W_MainMenu.W_MainMenu_C"))
  (bind _output_get (Variables|Default|SetMainMenu _returnvalue))
  (UserInterface|Viewport|AddtoViewport _output_get 0)
  (Input|SetInputModeGameOnly self)
  (EventDispatchers|BindEventtoAnimationFinished (Variables|Default|GetMainMenu) (delegate Custom|OpenGate)))

(event Input|ActionEvents|InputActionInteract
  (params (Key :type Key%20Structure :default "None"))
  (:Pressed
    (Utilities|FlowControl|Gate true
      (:Exit
        (Game|OpenLevel(byName) "Basecamp")))))

(fn ConstructionScript)